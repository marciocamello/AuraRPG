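; Flame pillar actor that flickers its fire light for as long as it is in play.
; On BeginPlay it randomly picks one of two intensity timelines, and each one picks again when it finishes, forming an endless randomized loop.
; Timeline updates feed ScaleFlameIntensity, which multiplies the curve value by BaseIntensity to set the FireLight intensity.
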(event Custom|StartTimelineTwo
  (bind _intensity (Timeline|FlameIntensityTimeline_2 PlayFromStart)
    (:Update
      (CallFunction|ScaleFlameIntensity _intensity))
    (:Finished
      (CallFunction|ChooseTimeline))))

(event Custom|StartTimelineOne
  (bind _intensity (Timeline|FlameIntensityTimeline_1 PlayFromStart)
    (:Update
      (CallFunction|ScaleFlameIntensity _intensity))
    (:Finished
      (CallFunction|ChooseTimeline))))

(event Custom|ChooseTimeline
  (switch int (Math|Random|RandomIntegerinRange 0 1)
    (:Default
      (CallFunction|StartTimelineTwo :!label _label))
    (:0
      (CallFunction|StartTimelineOne))
    (:1
      (goto _label))))

(event EventBeginPlay
  (CallFunction|ChooseTimeline))

(fn ConstructionScript)

(fn ScaleFlameIntensity
  (params (Intensity :type Float%20%28double-precision%29))
  (Rendering|Components|Light|SetIntensity (Variables|Default|GetFireLight) (* Intensity (Variables|Default|GetBaseIntensity))))