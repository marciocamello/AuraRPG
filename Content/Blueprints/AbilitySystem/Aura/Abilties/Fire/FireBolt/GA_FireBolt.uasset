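; GA_FireBolt is the Fire Bolt gameplay ability, which launches projectiles toward the point under the mouse.
; On activation it commits, takes mouse target data, turns the avatar toward the hit location and plays a random tagged attack montage.
; The montage's gameplay event triggers SpawnProjectiles, passing the hit actor as homing target.
; The ability ends when the montage completes, blends out or is stopped; an older SpawnProjectile call remains unconnected.
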(event Ability|EventActivateAbility
  (bind _returnvalue (Ability|GetAvatarActorfromActorInfo))
  (Ability|CommitAbility)
  (bind _datahandle (|TargetDataUnderMouse)
    (:ValidData
      (Variables|Default|SetProjectileTargetLocation (.Location (Collision|BreakHitResult (Ability|TargetData|GetHitResultfromTargetData _datahandle))))
      (Variables|Default|SetMouseHitActor (.HitActor (Collision|BreakHitResult (Ability|TargetData|GetHitResultfromTargetData _datahandle))))
      (Class|CombatInterface|UpdateFacingTarget(Message) _returnvalue (Variables|Default|GetProjectileTargetLocation))
      (bind _returnvalue_2 (Class|CombatInterface|GetAttackMontages(Message) _returnvalue))
      (Variables|Default|SetTaggedMontage (Class|AuraDamageGameplayAbility|GetRandomTaggedMontagefromArray _returnvalue_2))
      (|PlayMontageandWaitProxy "None" (.Montage (Utilities|Struct|BreakTaggedMontage (Variables|Default|GetTaggedMontage))) 1.0 "None" false 1.0 0.0 false
        (:then
          (Ability|Tasks|WaitGameplayEvent (.MontageTag (Utilities|Struct|BreakTaggedMontage (Variables|Default|GetTaggedMontage))) 0
            (:EventReceived
              (Class|AuraFireBolt|SpawnProjectiles (Variables|Default|GetProjectileTargetLocation) (Variables|Default|GetTaggedMontage) (Variables|Default|GetOverride%20Pitch) (Variables|Default|GetPitch%20Override) (Variables|Default|GetMouseHitActor)))))
        (:OnCompleted
          (Ability|EndAbility :!label _label))
        (:OnBlendOut
          (goto _label))
        (:OnInterrupted
          (goto _label))
        (:OnCancelled
          (goto _label))))))