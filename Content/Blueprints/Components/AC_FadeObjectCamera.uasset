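; Actor component that looks for objects in front of the player camera to swap them to a fade material.
; A looping timer starts at BeginPlay and periodically line-traces along the camera's forward vector, with debug drawing.
; On a hit, it creates a dynamic instance with Fade at zero but applies the parent FadeMaterialInstances to the actor's static mesh, leaving that instance unused.
; Original materials are never restored.
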(event Custom|FindActor
  (bind _returnvalue (Game|GetPlayerCameraManager 0))
  (bind _fadematerialinstances (Variables|Default|GetFadeMaterialInstances))
  (bind _rootcomponent (Variables|/Script/Engine.Actor|GetRootComponent _returnvalue))
  (bind _returnvalue_2 (Transformation|GetWorldLocation _rootcomponent))
  (bind (_outhit _returnvalue_3) (Collision|LineTraceByChannel _returnvalue_2 (+ _returnvalue_2 (* (Math|Vector|GetForwardVector (Transformation|GetWorldRotation _rootcomponent)) 2e+03)) "TraceTypeQuery3" false 0 "ForOneFrame"))
  (if _returnvalue_3
    (Rendering|Debug|DrawDebugSphere (.ImpactPoint (Collision|BreakHitResult _outhit)) 15.0 12 "(R=0.000000,G=1.000000,B=0.245103,A=1.000000)" 5.0)
    (bind _returnvalue_4 (Rendering|Material|CreateDynamicMaterialInstance _fadematerialinstances "None" "None" :!class /Script/Engine.KismetMaterialLibrary))
    (Rendering|Material|SetScalarParameterValue _returnvalue_4 "Fade" 0.0 :!class /Script/Engine.MaterialInstanceDynamic)
    (Rendering|Material|SetMaterial (Actor|GetComponentbyClass (.HitActor (Collision|BreakHitResult _outhit)) "/Script/Engine.StaticMeshComponent") 0 _fadematerialinstances)))

(event EventBeginPlay
  (bind _returnvalue (Utilities|Time|SetTimerbyEvent (delegate Custom|FindActor) 0.3 true))
  (Variables|Default|SetFindActorTimeHandle _returnvalue))