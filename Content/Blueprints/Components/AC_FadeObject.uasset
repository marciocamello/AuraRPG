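; Actor component for the top-down Aura character that fades out a static mesh in front of it and fades it back when clear.
; A looping timer line-traces along the character's forward vector, with debug drawing, to pick the mesh.
; It caches the original materials and swaps in dynamic fade-material instances.
; Fast timers step their "Fade" parameter, and FadeFinish restores the originals as fade-in nears completion.
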(event Custom|FindActor
  (bind _as_bp_aura_character_topdown (Variables|Default|GetAs%20BP%20Aura%20Character%20Topdown))
  (bind _rootcomponent (Variables|/Script/Engine.Actor|GetRootComponent _as_bp_aura_character_topdown))
  (bind _returnvalue (Transformation|GetWorldLocation _rootcomponent))
  (bind (_outhit _returnvalue_2) (Collision|LineTraceByChannel _returnvalue (+ _returnvalue (* (Math|Vector|GetForwardVector (Transformation|GetWorldRotation _rootcomponent)) 5e+02)) "TraceTypeQuery3" false 0 "ForOneFrame"))
  (if _returnvalue_2
    (Rendering|Debug|DrawDebugSphere (.ImpactPoint (Collision|BreakHitResult _outhit)) 5.0 12 "(R=0.000000,G=1.000000,B=0.245103,A=1.000000)" 1.0)
    (if (not (Variables|Default|GetbIsFadingOut%20))
      (Variables|FadeProperties|SetMesh (Actor|GetComponentbyClass (.HitActor (Collision|BreakHitResult _outhit)) "/Script/Engine.StaticMeshComponent"))
      (CallFunction|SetupMaterials)
      (CallFunction|EventFadeOut))
    (elif (Variables|Default|GetbIsFadingOut%20)
      (CallFunction|EventFadein))))

(event Custom|SetFadeOut
  (if (>= (Variables|FadeProperties|GetAnimationProgress%20) 0.0)
    (Variables|FadeProperties|SetAnimationProgress%20 (Math|Float|Max(Float) (- (Variables|FadeProperties|GetAnimationProgress%20) 0.01) 0.0))
    (if (<= (Variables|FadeProperties|GetAnimationProgress%20) 0.0)
      (Utilities|Time|ClearandInvalidateTimerbyHandle (Variables|Default|GetFadeOutTimer))
      (else
        (for _array_element (Variables|Default|GetDynamicMaterialInstances)
          (Rendering|Material|SetScalarParameterValue _array_element "Fade" (Variables|FadeProperties|GetAnimationProgress%20) :!class /Script/Engine.MaterialInstanceDynamic))))))

(event Custom|EventFadeOut
  (Variables|Default|SetbIsFadingOut%20 true)
  (CallFunction|SetMaterialtoDynamicInstances)
  (bind _returnvalue (Utilities|Time|SetTimerbyEvent (delegate Custom|SetFadeOut) 0.004 true))
  (Variables|Default|SetFadeOutTimer _returnvalue))

(event Custom|SetFadeIn
  (Variables|FadeProperties|SetAnimationProgress%20 (+ (Variables|FadeProperties|GetAnimationProgress%20) 0.01))
  (if (>= (Variables|FadeProperties|GetAnimationProgress%20) 1.0)
    (Utilities|Time|ClearandInvalidateTimerbyHandle (Variables|Default|GetFadeInTimer))
    (else
      (for _array_element (Variables|Default|GetDynamicMaterialInstances)
        (Rendering|Material|SetScalarParameterValue _array_element "Fade" (Variables|FadeProperties|GetAnimationProgress%20) :!class /Script/Engine.MaterialInstanceDynamic)
        (CallFunction|FadeFinish (Variables|FadeProperties|GetAnimationProgress%20))))))

(event Custom|EventFadeIn
  (Variables|Default|SetbIsFadingOut%20 false)
  (bind _returnvalue (Utilities|Time|SetTimerbyEvent (delegate Custom|SetFadeIn) 0.004 true))
  (Variables|Default|SetFadeInTimer _returnvalue))

(event EventBeginPlay
  (bind _asbp_aura_character_topdown (Utilities|Casting|CastToBP_AuraCharacter_Topdown (Components|GetOwner)))
  (Variables|Default|SetAs%20BP%20Aura%20Character%20Topdown _asbp_aura_character_topdown)
  (bind _returnvalue (Utilities|Time|SetTimerbyEvent (delegate Custom|FindActor) 0.3 true))
  (Variables|Default|SetFindActorTimeHandle _returnvalue))

(fn ResetMaterials
  (for (_array_element _array_index) (Variables|Default|GetOriginalMaterials)
    (bind _mesh (Variables|FadeProperties|GetMesh)
      (:then
        (Rendering|Material|SetMaterial _mesh _array_index _array_element))
      (:else))))

(fn FadeFinish
  (params (Intensity :type Float%20%28double-precision%29))
  (if (>= Intensity 0.99)
    (CallFunction|ResetMaterials)
    (Variables|FadeProperties|SetMesh 0)
    (if (Variables|FadeProperties|GetBlockVisibility)
      (Collision|SetCollisionResponsetoChannel (Variables|FadeProperties|GetMesh) "ECC_Visibility" "ECR_Block"))
    (elif (<= Intensity 0.0)
      (Variables|FadeProperties|SetMesh 0)
      (if (Variables|FadeProperties|GetBlockVisibility)
        (Collision|SetCollisionResponsetoChannel (Variables|FadeProperties|GetMesh) "ECC_Visibility" "ECR_Ignore")))))

(fn SetMaterialtoDynamicInstances
  (for (_array_element _array_index) (Variables|Default|GetDynamicMaterialInstances)
    (Rendering|Material|SetMaterial (Variables|FadeProperties|GetMesh) _array_index _array_element)))

(fn SetupMaterials
  (Utilities|Array|Clear (Variables|Default|GetDynamicMaterialInstances))
  (bind _output_get (Variables|Default|SetOriginalMaterials (Rendering|Material|GetMaterials (Variables|FadeProperties|GetMesh))))
  (for _array_element _output_get
    (bind _returnvalue (Rendering|Material|CreateDynamicMaterialInstance (Utilities|Array|Get(acopy) (Variables|FadeProperties|GetFadeMaterialInstances)) "None" "None" :!class /Script/Engine.KismetMaterialLibrary))
    (Utilities|Array|AddUnique (Variables|Default|GetDynamicMaterialInstances) _returnvalue)))